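; Spike hazard hitbox that triggers spike damage on the player's samurai character while it overlaps the actor.
; Overlap begin and end set a touching flag for the player pawn, and entry immediately calls the character's spike damage dispatcher.
; Tick repeats that call every frame while the flag is set, clearing it once Health reaches zero or below.
; An alternative touch check is left unconnected and never runs.
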(event EventBeginPlay)

(event Collision|EventActorBeginOverlap
  (params (OtherActor :type Actor%20Object%20Reference))
  (if (== OtherActor (Game|Player|GetPlayerPawn 0))
    (Variables|Default|SetIsTouchingSpikes true)
    (bind _asbp_samurai_character (Utilities|Casting|CastToBP_SamuraiCharacter (Game|GetPlayerCharacter 0)))
    (Default|CallSpikeDamageDispatcher _asbp_samurai_character)))

(event EventTick
  (params (DeltaSeconds :type Float%20%28single-precision%29))
  (if (Variables|Default|GetIsTouchingSpikes)
    (bind _asbp_samurai_character (Utilities|Casting|CastToBP_SamuraiCharacter (Game|GetPlayerCharacter 0)))
    (Default|CallSpikeDamageDispatcher _asbp_samurai_character)
    (if (<= (Variables|/Game/Blueprints/BP_SamuraiCharacter.BP_SamuraiCharacter_C|GetHealth _asbp_samurai_character) 0.0)
      (Variables|Default|SetIsTouchingSpikes false))))

(event Collision|EventActorEndOverlap
  (params (OtherActor :type Actor%20Object%20Reference))
  (if (== OtherActor (Game|Player|GetPlayerPawn 0))
    (Variables|Default|SetIsTouchingSpikes false)))

(fn ConstructionScript)